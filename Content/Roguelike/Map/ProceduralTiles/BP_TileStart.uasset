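; BP_TileStart is the start tile among the roguelike map's procedural tiles, placing the player into the level.
; On BeginPlay it spawns a PlayerStart above its own location and has the game mode restart the player there.
; It also spawns a BP_EnemyCharacter offset to the side, marked as a debugging aid.
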(event `self.ReceiveBeginPlay`
  ;[1 1 1] Spawn Payer Start
  (bind _returnvalue (`|SpawnActorFromClass` "/Script/Engine.PlayerStart" (`KismetMathLibrary.Conv_VectorToTransform` (+ (`self.K2_GetActorLocation`) (0.0 0.0 200.0))) "Undefined" "OverrideRootScale" null null))
  ;[1 1 1] Restart Player
  (`GameModeBase.RestartPlayerAtPlayerStart` (`/Game/Roguelike/Blueprints/BP_FunctionLibrary.GetGameModeBP`) (`/Game/Roguelike/Blueprints/BP_FunctionLibrary.GetPlayerControllerBP`) _returnvalue)
  ;[1 1 1] Spawn AI Character (Debugging)
  (`|SpawnActorFromClass` "/Game/Roguelike/Characters/Enemy/BP_EnemyCharacter.BP_EnemyCharacter_C" (`KismetMathLibrary.Conv_VectorToTransform` (+ (`self.K2_GetActorLocation`) (0.0 500.0 200.0))) "Undefined" "OverrideRootScale" null null))

(fn `UserConstructionScript`)
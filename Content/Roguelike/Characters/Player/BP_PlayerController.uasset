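; Player controller for the roguelike that drives click-to-move movement and owns the in-game HUD.
; On first possession it caches the BP_PlayerCharacter, then creates and shows the WB_HUD widget, whose visibility ShowHUD toggles.
; While CharacterMove is held, a gate on Tick runs MoveToCursor, which traces under the cursor and uses SimpleMoveToLocation for points beyond a minimum distance from the pawn.
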(event `self.ReceivePossess`
  (params (PossessedPawn :type "Pawn Object Reference"))
  ;[0.6045 0.5568 1] Possess
  (`/Engine/EditorBlueprintResources/StandardMacros.DoOnce` false
    (:`Completed`
      (bind _asbp_player_character (cast `/Game/Roguelike/Characters/Player/BP_PlayerCharacter` PossessedPawn))
      (set `self.PlayerCharacter` _asbp_player_character)
      (`self.CreateHUD`))))

(event `CreateHUD`
  ;[0.1293 0.2624 0.4072] HUD
  (`/Engine/EditorBlueprintResources/StandardMacros.IsValid` (`self.InGameHUD`)
    (:`Is Valid`
      _)
    (:`Is Not Valid`
      (bind _returnvalue (`|CreateWidget` "/Game/Roguelike/UI/In-Game/WB_HUD.WB_HUD_C" self))
      (bind _output_get (set `self.InGameHUD` _returnvalue))
      (`UserWidget.AddToViewport` _output_get 0)))
  (`self.ShowHUD` true))

(event `ShowHUD`
  (params (Visible :type Boolean))
  (bind _ingamehud (`self.InGameHUD`))
  ;[0.1293 0.2624 0.4072] HUD
  (`/Engine/EditorBlueprintResources/StandardMacros.IsValid` _ingamehud
    (:`Is Valid`
      (`Widget.SetVisibility` _ingamehud (select `bool` Visible :`false` "Hidden" :`true` "SelfHitTestInvisible" :!type "ESlateVisibility Enum")))))

(event `self.ReceiveTick`
  (params (DeltaSeconds :type "Float (single-precision)"))
  ;[0.3808 0.8696 1] Movements
  (`/Engine/EditorBlueprintResources/StandardMacros.Gate` true :!label _label
    (:`Exit`
      (`self.MoveToCursor`))))

(event `InputAction|CharacterMove`
  (params (Key :type "Key Structure"))
  ;[0.3808 0.8696 1] Movements
  (:`Pressed`
    (goto _label :!via `Open`))
  (:`Released`
    (goto _label :!via `Close`)))

(fn `MoveToCursor`
  (bind (_bblockinghit _binitialoverlap _time _distance _location) (`GameplayStatics.BreakHitResult` (`self.GetHitResultUnderCursorByChannel` "TraceTypeQuery1")))
  (if (>= (`KismetMathLibrary.VSize` (- (`self.K2_GetActorLocation` (`self.K2_GetPawn`)) _location)) (`self.MinClickDistance`))
    (`AIBlueprintHelperLibrary.SimpleMoveToLocation` self _location)))

(fn `UserConstructionScript`)
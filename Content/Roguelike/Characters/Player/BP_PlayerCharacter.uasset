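; Player character Blueprint for the roguelike, built on the Gameplay Ability System with most logic inherited from its parent class.
; The AbilityInput_1 press triggers DoSkillAttack.
; The rest is debug output: damage and health-change events print their values to screen.
; Tick recalculates max health every frame and prints an attribute read from the Ability System Component, labelled as health.
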(event `InputAction|AbilityInput_1`
  (params (Key :type "Key Structure"))
  ;[0.5515 0.4912 1] Ability Inputs
  (:`Pressed`
    (`self.DoSkillAttack`)))

(event `InputAction|AbilityInput_2`
  (params (Key :type "Key Structure"))
  ;[0.5515 0.4912 1] Ability Inputs
)

(event `InputAction|AbilityInput_3`
  (params (Key :type "Key Structure"))
  ;[0.5515 0.4912 1] Ability Inputs
)

(event `InputAction|AbilityInput_4`
  (params (Key :type "Key Structure"))
  ;[0.5515 0.4912 1] Ability Inputs
)

(event `InputAction|AbilityInput_5`
  (params (Key :type "Key Structure"))
  ;[0.5515 0.4912 1] Ability Inputs
)

(event `InputAction|AbilityInput_6`
  (params (Key :type "Key Structure"))
  ;[0.5515 0.4912 1] Ability Inputs
)

(event `InputAction|AbilityInput_7`
  (params (Key :type "Key Structure"))
  ;[0.5515 0.4912 1] Ability Inputs
)

(event `InputAction|AbilityInput_8`
  (params (Key :type "Key Structure"))
  ;[0.5515 0.4912 1] Ability Inputs
)

(event `self.OnDamaged`
  (params (DamageAmount :type "Float (single-precision)") (HitInfo :type "HitResult Structure (by ref)") (DamageTags :type "GameplayTagContainer Structure (by ref)") (InstigatorCharacter :type "RPGCharacterBase Object Reference") (DamageCauser :type "Actor Object Reference"))
  ;[1 1 1] Debugging
  (`KismetSystemLibrary.PrintString` "Damage Receive")
  (`KismetSystemLibrary.PrintString` (`KismetStringLibrary.Conv_DoubleToString` DamageAmount)))

(event `self.OnHealthChanged`
  (params (DeltaValue :type "Float (single-precision)") (EventTags :type "GameplayTagContainer Structure (by ref)"))
  ;[1 1 1] Debugging
  (`KismetSystemLibrary.PrintString` "Health Reduced")
  (`KismetSystemLibrary.PrintString` (`KismetStringLibrary.Conv_DoubleToString` DeltaValue)))

(event `self.ReceiveTick`
  (params (DeltaSeconds :type "Float (single-precision)"))
  ;[1 1 1] Print Health From Attribute Set
  (`self.CalculateMaxHealth`)
  (`KismetSystemLibrary.PrintString` (`KismetStringLibrary.Conv_DoubleToString` (`.ReturnValue` (`AbilitySystemBlueprintLibrary.GetFloatAttributeFromAbilitySystemComponent` (`AbilitySystemBlueprintLibrary.GetAbilitySystemComponent` self) (struct :`AttributeName` "MaxHealth" :`Attribute` "/Script/RoguelikeGame.RPGAttributeSet:MaxHealth"))))))

(fn `UserConstructionScript`
  (`parent.UserConstructionScript`))
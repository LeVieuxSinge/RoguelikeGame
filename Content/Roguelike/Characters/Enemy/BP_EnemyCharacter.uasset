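; BP_EnemyCharacter is an enemy character Blueprint for the roguelike game, with minimal logic of its own.
; On Tick it reads a float attribute from its Ability System Component and prints it, apparently as debug output.
; UpdateWalkSpeed sets the Character Movement max walk speed to a given value, with no caller in this graph.
; The construction script only calls its parent.
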(event `self.ReceiveTick`
  (params (DeltaSeconds :type "Float (single-precision)"))
  (`KismetSystemLibrary.PrintString` (`KismetStringLibrary.Conv_DoubleToString` (`.ReturnValue` (`AbilitySystemBlueprintLibrary.GetFloatAttributeFromAbilitySystemComponent` (`AbilitySystemBlueprintLibrary.GetAbilitySystemComponent` self) (struct :`AttributeName` "Health" :`Attribute` "/Script/RoguelikeGame.RPGAttributeSet:Health"))))))

(fn `UpdateWalkSpeed`
  (params (NewWalkSpeed :type "Float (double-precision)"))
  (set `CharacterMovementComponent.MaxWalkSpeed` NewWalkSpeed (`self.CharacterMovement`)))

(fn `UserConstructionScript`
  (`parent.UserConstructionScript`))
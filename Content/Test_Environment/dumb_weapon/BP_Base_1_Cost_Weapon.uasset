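; Base weapon for the 1-cost tier that rolls itself on BeginPlay from a random row of 1_Cost_Weapon_Data_Table.
; Each of its five modifier slots names a category, which resolves to a random modifier name, though a few melee and shield cases always pick the first entry.
; CreateMODArray adds only fire, lightning and cold damage increases to MOD.
; The rolled names are written back into WeaponInfo, and the row's skeletal mesh is applied.
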(event `self.ReceiveBeginPlay`
  (bind _outrownames (`DataTableFunctionLibrary.GetDataTableRowNames` "/Game/Test_Environment/dumb_weapon/1_Cost_Weapon_Data_Table.1_Cost_Weapon_Data_Table"))
  (bind _returnvalue (`|GetDataTableRow` "/Game/Test_Environment/dumb_weapon/1_Cost_Weapon_Data_Table.1_Cost_Weapon_Data_Table" (`|GetArrayItem` _outrownames (`KismetMathLibrary.RandomInteger` 27)))
    (:`then`
      (bind _output_get (set `self.WeaponInfo` _returnvalue))
      (bind (_weaponname _damagestyle _weapontype _elementtype _candophysicaldamage _candofiredamage _candolightningdamage _candoicedamage _physicaldamagemultiplier _firedamagemultiplier _lightningdamagemultiplier _colddamagemultiplier _distancemultiplier _projectilespeed _areaofeffect _attackspeed _criticalchance _criticaldamagemultiplier _onhitchance _onhitdamagemultiplier _modifier_1 _modifier_2 _modifier_3 _modifier_4 _modifier_5 _mesh _cost) (break `/Game/Test_Environment/dumb_weapon/FWeaponInfo` _output_get))
      (switch `|SwitchEnum` _modifier_1
        (:`NewEnumerator0`
          (set `self.Modifier1` "None"))
        (:`NewEnumerator1`
          (bind _output_get_2 (set `self.MeleeModifiers` (cast `` (`KismetMathLibrary.Conv_IntToByte` (`KismetMathLibrary.RandomIntegerInRange` 0 3)))))
          (set `self.Modifier1` (`|GetEnumeratorName` _output_get_2)))
        (:`NewEnumerator4`
          (bind _output_get_3 (set `self.ProjectileModifiers` (cast `` (`KismetMathLibrary.Conv_IntToByte` (`KismetMathLibrary.RandomIntegerInRange` 0 3)))))
          (set `self.Modifier1` (`|GetEnumeratorName` _output_get_3)))
        (:`NewEnumerator3`
          (bind _output_get_4 (set `self.ZoneModifiers` (cast `` (`KismetMathLibrary.Conv_IntToByte` (`KismetMathLibrary.RandomIntegerInRange` 0 3)))))
          (set `self.Modifier1` (`|GetEnumeratorName` _output_get_4)))
        (:`NewEnumerator5`
          (bind _output_get_5 (set `self.ShieldModifiers` (cast `` (`KismetMathLibrary.Conv_IntToByte` (`KismetMathLibrary.RandomIntegerInRange` 0 3)))))
          (set `self.Modifier1` (`|GetEnumeratorName` _output_get_5)))
        (:`NewEnumerator6`
          (bind _output_get_6 (set `self.ArmorModifier` (cast `` (`KismetMathLibrary.Conv_IntToByte` (`KismetMathLibrary.RandomIntegerInRange` 0 3)))))
          (set `self.Modifier1` (`|GetEnumeratorName` _output_get_6)))
        (:`NewEnumerator7`
          (bind _output_get_7 (set `self.BootsModifier` (cast `` (`KismetMathLibrary.Conv_IntToByte` (`KismetMathLibrary.RandomIntegerInRange` 0 3)))))
          (set `self.Modifier1` (`|GetEnumeratorName` _output_get_7)))
        (:`NewEnumerator2`
          (bind _output_get_8 (set `self.GlobalModifiers` (cast `` (`KismetMathLibrary.Conv_IntToByte` (`KismetMathLibrary.RandomIntegerInRange` 0 3)))))
          (set `self.Modifier1` (`|GetEnumeratorName` _output_get_8))))
      (switch `|SwitchEnum` _modifier_2
        (:`NewEnumerator0`
          (set `self.Modifier2` "None"))
        (:`NewEnumerator1`
          (bind _output_get_9 (set `self.MeleeModifiers` (cast `` (`KismetMathLibrary.Conv_IntToByte` (`KismetMathLibrary.RandomIntegerInRange` 0 3)))))
          (set `self.Modifier2` (`|GetEnumeratorName` _output_get_9)))
        (:`NewEnumerator4`
          (bind _output_get_10 (set `self.ProjectileModifiers` (cast `` (`KismetMathLibrary.Conv_IntToByte` (`KismetMathLibrary.RandomIntegerInRange` 0 3)))))
          (set `self.Modifier2` (`|GetEnumeratorName` _output_get_10)))
        (:`NewEnumerator3`
          (bind _output_get_11 (set `self.ZoneModifiers` (cast `` (`KismetMathLibrary.Conv_IntToByte` (`KismetMathLibrary.RandomIntegerInRange` 0 3)))))
          (set `self.Modifier2` (`|GetEnumeratorName` _output_get_11)))
        (:`NewEnumerator5`
          (bind _output_get_12 (set `self.ShieldModifiers` (cast `` (`KismetMathLibrary.Conv_IntToByte` (`KismetMathLibrary.RandomIntegerInRange` 0 3)))))
          (set `self.Modifier2` (`|GetEnumeratorName` _output_get_12)))
        (:`NewEnumerator6`
          (bind _output_get_13 (set `self.ArmorModifier` (cast `` (`KismetMathLibrary.Conv_IntToByte` (`KismetMathLibrary.RandomIntegerInRange` 0 3)))))
          (set `self.Modifier2` (`|GetEnumeratorName` _output_get_13)))
        (:`NewEnumerator7`
          (bind _output_get_14 (set `self.BootsModifier` (cast `` (`KismetMathLibrary.Conv_IntToByte` (`KismetMathLibrary.RandomIntegerInRange` 0 3)))))
          (set `self.Modifier2` (`|GetEnumeratorName` _output_get_14)))
        (:`NewEnumerator2`
          (bind _output_get_15 (set `self.GlobalModifiers` (cast `` (`KismetMathLibrary.Conv_IntToByte` (`KismetMathLibrary.RandomIntegerInRange` 0 3)))))
          (set `self.Modifier2` (`|GetEnumeratorName` _output_get_15))))
      (switch `|SwitchEnum` _modifier_3
        (:`NewEnumerator0`
          (set `self.Modifier3` "None"))
        (:`NewEnumerator1`
          (bind _output_get_16 (set `self.MeleeModifiers` (cast `` (`KismetMathLibrary.Conv_IntToByte` 0))))
          (set `self.Modifier3` (`|GetEnumeratorName` _output_get_16)))
        (:`NewEnumerator4`
          (bind _output_get_17 (set `self.ProjectileModifiers` (cast `` (`KismetMathLibrary.Conv_IntToByte` (`KismetMathLibrary.RandomIntegerInRange` 0 3)))))
          (set `self.Modifier3` (`|GetEnumeratorName` _output_get_17)))
        (:`NewEnumerator3`
          (bind _output_get_18 (set `self.ZoneModifiers` (cast `` (`KismetMathLibrary.Conv_IntToByte` (`KismetMathLibrary.RandomIntegerInRange` 0 3)))))
          (set `self.Modifier3` (`|GetEnumeratorName` _output_get_18)))
        (:`NewEnumerator5`
          (bind _output_get_19 (set `self.ShieldModifiers` (cast `` (`KismetMathLibrary.Conv_IntToByte` (`KismetMathLibrary.RandomIntegerInRange` 0 3)))))
          (set `self.Modifier3` (`|GetEnumeratorName` _output_get_19)))
        (:`NewEnumerator6`
          (bind _output_get_20 (set `self.ArmorModifier` (cast `` (`KismetMathLibrary.Conv_IntToByte` (`KismetMathLibrary.RandomIntegerInRange` 0 3)))))
          (set `self.Modifier3` (`|GetEnumeratorName` _output_get_20)))
        (:`NewEnumerator7`
          (bind _output_get_21 (set `self.BootsModifier` (cast `` (`KismetMathLibrary.Conv_IntToByte` (`KismetMathLibrary.RandomIntegerInRange` 0 3)))))
          (set `self.Modifier3` (`|GetEnumeratorName` _output_get_21)))
        (:`NewEnumerator2`
          (bind _output_get_22 (set `self.GlobalModifiers` (cast `` (`KismetMathLibrary.Conv_IntToByte` (`KismetMathLibrary.RandomIntegerInRange` 0 3)))))
          (set `self.Modifier3` (`|GetEnumeratorName` _output_get_22))))
      (switch `|SwitchEnum` _modifier_4
        (:`NewEnumerator0`
          (set `self.Modifier4` "None"))
        (:`NewEnumerator1`
          (bind _output_get_23 (set `self.MeleeModifiers` (cast `` (`KismetMathLibrary.Conv_IntToByte` (`KismetMathLibrary.RandomIntegerInRange` 0 3)))))
          (set `self.Modifier4` (`|GetEnumeratorName` _output_get_23)))
        (:`NewEnumerator4`
          (bind _output_get_24 (set `self.ProjectileModifiers` (cast `` (`KismetMathLibrary.Conv_IntToByte` (`KismetMathLibrary.RandomIntegerInRange` 0 3)))))
          (set `self.Modifier4` (`|GetEnumeratorName` _output_get_24)))
        (:`NewEnumerator3`
          (bind _output_get_25 (set `self.ZoneModifiers` (cast `` (`KismetMathLibrary.Conv_IntToByte` (`KismetMathLibrary.RandomIntegerInRange` 0 3)))))
          (set `self.Modifier4` (`|GetEnumeratorName` _output_get_25)))
        (:`NewEnumerator5`
          (bind _output_get_26 (set `self.ShieldModifiers` (cast `` (`KismetMathLibrary.Conv_IntToByte` 0))))
          (set `self.Modifier4` (`|GetEnumeratorName` _output_get_26)))
        (:`NewEnumerator6`
          (bind _output_get_27 (set `self.ArmorModifier` (cast `` (`KismetMathLibrary.Conv_IntToByte` (`KismetMathLibrary.RandomIntegerInRange` 0 3)))))
          (set `self.Modifier4` (`|GetEnumeratorName` _output_get_27)))
        (:`NewEnumerator7`
          (bind _output_get_28 (set `self.BootsModifier` (cast `` (`KismetMathLibrary.Conv_IntToByte` (`KismetMathLibrary.RandomIntegerInRange` 0 3)))))
          (set `self.Modifier4` (`|GetEnumeratorName` _output_get_28)))
        (:`NewEnumerator2`
          (bind _output_get_29 (set `self.GlobalModifiers` (cast `` (`KismetMathLibrary.Conv_IntToByte` (`KismetMathLibrary.RandomIntegerInRange` 0 3)))))
          (set `self.Modifier4` (`|GetEnumeratorName` _output_get_29))))
      (switch `|SwitchEnum` _modifier_5
        (:`NewEnumerator0`
          (set `self.Modifier5` "None"))
        (:`NewEnumerator1`
          (bind _output_get_30 (set `self.MeleeModifiers` 0))
          (set `self.Modifier5` (`|GetEnumeratorName` _output_get_30)))
        (:`NewEnumerator4`
          (bind _output_get_31 (set `self.ProjectileModifiers` (cast `` (`KismetMathLibrary.Conv_IntToByte` (`KismetMathLibrary.RandomIntegerInRange` 0 3)))))
          (set `self.Modifier5` (`|GetEnumeratorName` _output_get_31)))
        (:`NewEnumerator3`
          (bind _output_get_32 (set `self.ZoneModifiers` (cast `` (`KismetMathLibrary.Conv_IntToByte` (`KismetMathLibrary.RandomIntegerInRange` 0 3)))))
          (set `self.Modifier5` (`|GetEnumeratorName` _output_get_32)))
        (:`NewEnumerator5`
          (bind _output_get_33 (set `self.ShieldModifiers` (cast `` (`KismetMathLibrary.Conv_IntToByte` (`KismetMathLibrary.RandomIntegerInRange` 0 3)))))
          (set `self.Modifier5` (`|GetEnumeratorName` _output_get_33)))
        (:`NewEnumerator6`
          (bind _output_get_34 (set `self.ArmorModifier` (cast `` (`KismetMathLibrary.Conv_IntToByte` (`KismetMathLibrary.RandomIntegerInRange` 0 3)))))
          (set `self.Modifier5` (`|GetEnumeratorName` _output_get_34)))
        (:`NewEnumerator7`
          (bind _output_get_35 (set `self.BootsModifier` (cast `` (`KismetMathLibrary.Conv_IntToByte` (`KismetMathLibrary.RandomIntegerInRange` 0 3)))))
          (set `self.Modifier5` (`|GetEnumeratorName` _output_get_35)))
        (:`NewEnumerator2`
          (bind _output_get_36 (set `self.GlobalModifiers` (cast `` (`KismetMathLibrary.Conv_IntToByte` (`KismetMathLibrary.RandomIntegerInRange` 0 3)))))
          (set `self.Modifier5` (`|GetEnumeratorName` _output_get_36))))
      (`self.Create_MOD_Array` self (`self.Modifier1`) (`self.Modifier2`) (`self.Modifier3`) (`self.Modifier4`) (`self.Modifier5`))
      (set `self.WeaponInfo` (make `/Game/Test_Environment/dumb_weapon/FWeaponInfo` _weaponname _damagestyle _weapontype _elementtype _candophysicaldamage _candofiredamage _candolightningdamage _candoicedamage _physicaldamagemultiplier _firedamagemultiplier _lightningdamagemultiplier _colddamagemultiplier _distancemultiplier _projectilespeed _areaofeffect _attackspeed _criticalchance _criticaldamagemultiplier _onhitchance _onhitdamagemultiplier 0 0 0 0 0 _mesh _cost (`self.Modifier1`) (`self.Modifier2`) (`self.Modifier3`) (`self.Modifier4`) (`self.Modifier5`)))
      (`SkinnedMeshComponent.SetSkinnedAssetAndUpdate` (`self.SkeletalMesh`) _mesh true))))

(fn `Create_MOD_Array`
  (params (MOD1 :type Name) (MOD2 :type Name) (MOD3 :type Name) (MOD4 :type Name) (MOD5 :type Name))
  (for _array_element (`|MakeArray` MOD1 MOD2 MOD3 MOD4 MOD5)
    (switch `name` _array_element
      (:`Increase Fire Damage`
        (`KismetArrayLibrary.Array_Add` (`self.MOD`) (`self.Increase Fire Damage`)))
      (:`Increase Lightning Damage`
        (`KismetArrayLibrary.Array_Add` (`self.MOD`) (`self.Increase_Lightning Damage`)))
      (:`Increase Cold Damage`
        (`KismetArrayLibrary.Array_Add` (`self.MOD`) (`self.Increase_Cold Damage`))))))

(fn `UserConstructionScript`)
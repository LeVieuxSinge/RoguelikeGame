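; Base weapon actor that rolls a random weapon definition from the 1-cost weapon data table.
; On BeginPlay it picks a row name using a hardcoded random range of 27 and stores the found row in WeaponInfo.
; It then loops over the five modifier fields with an empty body, and a string check for MeleeModifier sits unconnected.
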(event `self.ReceiveBeginPlay`
  (bind _outrownames (`DataTableFunctionLibrary.GetDataTableRowNames` "/Game/Test_Environment/dumb_weapon/1_Cost_Weapon_Data_Table.1_Cost_Weapon_Data_Table"))
  (bind _returnvalue (`|GetDataTableRow` "/Game/Test_Environment/dumb_weapon/1_Cost_Weapon_Data_Table.1_Cost_Weapon_Data_Table" (`|GetArrayItem` _outrownames (`KismetMathLibrary.RandomInteger` 27)))
    (:`then`
      (bind _output_get (set `self.WeaponInfo` _returnvalue))
      (bind (_weaponname _damagestyle _weapontype _elementtype _candophysicaldamage _candofiredamage _candolightningdamage _candoicedamage _physicaldamagemultiplier _firedamagemultiplier _lightningdamagemultiplier _colddamagemultiplier _distancemultiplier _projectilespeed _areaofeffect _attackspeed _criticalchance _criticaldamagemultiplier _onhitchance _onhitdamagemultiplier _modifier_1 _modifier_2 _modifier_3 _modifier_4 _modifier_5) (break `/Game/Test_Environment/dumb_weapon/FWeaponInfo` _output_get))
      (for _array_element (`|MakeArray` _modifier_1 _modifier_2 _modifier_3 _modifier_4 _modifier_5)
        _))))

(fn `UserConstructionScript`
  (`parent.UserConstructionScript`))
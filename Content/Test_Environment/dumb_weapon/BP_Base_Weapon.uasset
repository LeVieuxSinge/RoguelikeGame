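; BP_Base_Weapon is a test weapon Blueprint that prototypes a random weapon roll on BeginPlay.
; Nested percentage-style rolls against fixed thresholds lead, when all fail, to a random row lookup in the 1-cost weapon data table.
; The first check, RandomInteger(1) == 0, is always true and its branch is empty, so the lookup never runs.
; The fetched row is unused, as is MainHand.
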(event `self.ReceiveBeginPlay`
  (if (== (`KismetMathLibrary.RandomInteger` 1) 0)
    _
    (elif (<= (`KismetMathLibrary.RandomInteger` 99) (+ 5 0))
      _
      (elif (<= (- (`KismetMathLibrary.RandomInteger` 99) 0) (+ 20 0))
        _
        (elif (not (<= (- (`KismetMathLibrary.RandomInteger` 99) (+ 20 0)) (+ 50 0)))
          (bind _outrownames (`DataTableFunctionLibrary.GetDataTableRowNames` "/Game/Test_Environment/dumb_weapon/1_Cost_Weapon_Data_Table.1_Cost_Weapon_Data_Table"))
          (`|GetDataTableRow` "/Game/Test_Environment/dumb_weapon/1_Cost_Weapon_Data_Table.1_Cost_Weapon_Data_Table" (`|GetArrayItem` _outrownames (`KismetMathLibrary.RandomInteger` 27))))))))

(fn `UserConstructionScript`)